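; Player-steered snake head that moves forward constantly and grows a tail of spawned BP_Tail segments.
; Each tick it applies a velocity-change impulse to Head and adjusts yaw from input values or mobile turn flags.
; AddBody spawns a segment at SpawnPoint, records its sphere, then snaps SpawnPoint onto it for the next.
; Skin rebuilds a spline through the body positions every tick and stretches spline meshes along it, recreating them when the count changes.
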(event `self.ReceiveBeginPlay`
  (bind _index (`self.Index`))
  (`KismetArrayLibrary.Array_Set` (`self.Bodys`) _index (`self.Head`) true)
  (set `self.Index` (+ _index 1))
  (for _ (range (+ (`self.StartBodys`) 1))
    (`self.AddBody`)))

(event `self.ReceiveTick`
  (params (DeltaSeconds :type "Float (single-precision)"))
  (set `self.DeltaSeconds` DeltaSeconds)
  (`|ExecutionSequence`
    (:`then_0`
      (`self.MoveForward`))
    (:`then_1`
      (`self.RotateRight`))
    (:`then_2`
      (`self.RotateLeft`))
    (:`then_3`
      (`self.Skin`))
    (:`then_4`
      (`self.RotateLeftMobile`))
    (:`then_5`
      (`self.RotateRightMobile`))))

(event `MoveForward`
  ;[1 1 1] Move Forward
  (`PrimitiveComponent.AddImpulse` (`self.Head`) (* (`SceneComponent.GetForwardVector` (`self.Direction`)) (`self.MovementSpeed`)) "None" true))

(event `RotateRight`
  (bind (_returnvalue_roll _returnvalue_pitch _returnvalue_yaw) (`KismetMathLibrary.BreakRotator` (`SceneComponent.K2_GetComponentRotation` (`self.Head`))))
  ;[1 1 1] Rotate Right
  (if (> (`self.GetInputAxisValue`) 0.0)
    (`SceneComponent.K2_SetRelativeRotation` (`self.Head`) (`KismetMathLibrary.MakeRotator` _returnvalue_roll _returnvalue_pitch (+ _returnvalue_yaw (`self.RotationSpeed`))) false false)))

(event `RotateRightMobile`
  (bind (_returnvalue_roll _returnvalue_pitch _returnvalue_yaw) (`KismetMathLibrary.BreakRotator` (`SceneComponent.K2_GetComponentRotation` (`self.Head`))))
  (if (`self.RotRight`)
    (`SceneComponent.K2_SetRelativeRotation` (`self.Head`) (`KismetMathLibrary.MakeRotator` _returnvalue_roll _returnvalue_pitch (+ _returnvalue_yaw (`self.RotationSpeed`))) false false)))

(event `RotateLeft`
  (bind (_returnvalue_roll _returnvalue_pitch _returnvalue_yaw) (`KismetMathLibrary.BreakRotator` (`SceneComponent.K2_GetComponentRotation` (`self.Head`))))
  ;[1 1 1] Rotate Left
  (if (> (`self.GetInputAxisValue`) 0.0)
    (`SceneComponent.K2_SetRelativeRotation` (`self.Head`) (`KismetMathLibrary.MakeRotator` _returnvalue_roll _returnvalue_pitch (- _returnvalue_yaw (`self.RotationSpeed`))) false false)))

(event `RotateLeftMobile`
  (bind (_returnvalue_roll _returnvalue_pitch _returnvalue_yaw) (`KismetMathLibrary.BreakRotator` (`SceneComponent.K2_GetComponentRotation` (`self.Head`))))
  (if (`self.RotLeft`)
    (`SceneComponent.K2_SetRelativeRotation` (`self.Head`) (`KismetMathLibrary.MakeRotator` _returnvalue_roll _returnvalue_pitch (- _returnvalue_yaw (`self.RotationSpeed`))) false false)))

(event `AddBody`
  (bind _index (`self.Index`))
  ;[1 1 1] Add Body
  (bind _returnvalue (`|SpawnActorFromClass` "/Game/Blueprints/BP_Tail.BP_Tail_C" (`SceneComponent.K2_GetComponentToWorld` (`self.SpawnPoint`)) "AlwaysSpawn" "OverrideRootScale" null null))
  (`/Game/Blueprints/BP_Tail.SetFollowing` _returnvalue self)
  (set `self.TailEnd` _returnvalue)
  (bind _sphere (`/Game/Blueprints/BP_Tail.Sphere` _returnvalue))
  (set `self.AttacheComp` _sphere)
  (`KismetArrayLibrary.Array_Set` (`self.Bodys`) _index _sphere true)
  (set `self.Index` (+ _index 1))
  (`self.ResetSpawnPoint`))

(event `ResetSpawnPoint`
  ;[1 1 1] ResetSpawnPoint
  (`SceneComponent.K2_AttachToComponent` (`self.SpawnPoint`) (`self.AttacheComp`) "None" "SnapToTarget" "SnapToTarget" "SnapToTarget" true))

(event `Skin`
  (bind _spm_s (`self.SPM´s`))
  (bind _spm_s_2 (`self.SPM´s`))
  (bind _spline (`self.Spline`))
  ;[0.4768 1 0.2543] Skin
  (for (_array_element _array_index) (`self.Bodys`)
    (`KismetArrayLibrary.Array_Set` (`self.PointPositions`) _array_index (`SceneComponent.K2_GetComponentLocation` _array_element) true)
    (`SplineComponent.SetSplinePoints` (`self.Spline`) (`self.PointPositions`) "World" true)
    (for _index (range 1 (+ (`SplineComponent.GetNumberOfSplinePoints` (`self.Spline`)) 1))
      (if (!= (`KismetArrayLibrary.Array_Length` (`self.PointPositions`)) (`KismetArrayLibrary.Array_Length` (`self.SPM´s`)))
        (for _array_element_2 _spm_s
          (`ActorComponent.K2_DestroyComponent` _array_element_2))
        (`KismetArrayLibrary.Array_Clear` _spm_s)
        (for _ (range 1 (+ (`SplineComponent.GetNumberOfSplinePoints` (`self.Spline`)) 1))
          (bind _returnvalue (`AddComponent|NODE_AddSplineMeshComponent-0` :`bManualAttachment` true))
          (`KismetArrayLibrary.Array_Add` _spm_s_2 _returnvalue)))
      (bind _returnvalue_2 (- _index 1))
      (bind (_location _tangent) (`SplineComponent.GetLocationAndTangentAtSplinePoint` _spline _returnvalue_2 "World"))
      (bind (_location_2 _tangent_2) (`SplineComponent.GetLocationAndTangentAtSplinePoint` _spline _index "World"))
      (`SplineMeshComponent.SetStartAndEnd` (`|GetArrayItem` _spm_s_2 _returnvalue_2) _location _tangent _location_2 _tangent_2 true))))

(event `SetTailScale`
  (`SplineMeshComponent.SetEndScale` (`|GetArrayItem` (`self.SPM´s`) (`self.Index`)) (0.0 0.0) true))

(fn `UserConstructionScript`
  (set `self.TailEnd` self))