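; BP_Tail is a snake tail segment that trails the segment in front of it.
; SetFollowing stores the snake head and takes its current TailEnd as the segment to follow.
; Each Tick, FollowTailInFront uses VInterpTo at FollowSpeed to ease the Sphere component toward that target's actor location, teleporting without sweep.
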(event `self.ReceiveTick`
  (params (DeltaSeconds :type "Float (single-precision)"))
  (set `self.DeltaSeconds` DeltaSeconds)
  (`self.FollowTailInFront`))

(event `FollowTailInFront`
  (bind _sphere (`self.Sphere`))
  ;[1 1 1] FollowTailInFront
  (`SceneComponent.K2_SetWorldLocation` _sphere (`KismetMathLibrary.VInterpTo` (`SceneComponent.K2_GetComponentLocation` _sphere) (`self.K2_GetActorLocation` (`self.TailInFront`)) (`self.DeltaSeconds`) (`self.FollowSpeed`)) false true))

(event `SetFollowing`
  (params (SnakeHead :type "/Game/Blueprints/BP_SnakeHead Object Reference"))
  ;[1 1 1] SetFollow
  (bind _output_get (set `self.SnakeHead` SnakeHead))
  (set `self.TailInFront` (`/Game/Blueprints/BP_SnakeHead.TailEnd` _output_get)))

(fn `UserConstructionScript`)